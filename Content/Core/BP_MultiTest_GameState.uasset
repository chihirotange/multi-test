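; BP_MultiTest_GameState is a game state that keeps a registry of current players and announces new ones to registered observers.
; RegisterPlayertoRegistry adds each player uniquely and calls OnNewPlayerAdded on every observer only when the player is new.
; A binding to each player's OnEndPlay removes it from the registry without notifying observers.
; GetAllCurrentPlayers exposes the list, as observers receive no replay of earlier registrations.
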(event Custom|OnPlayerEndplay
  (params (Actor :type Actor%20Object%20Reference) (EndPlayReason :type EEndPlayReason%20Enum :default "Destroyed"))
  (Utilities|Array|RemoveItem (Variables|Default|GetPlayerArrays) Actor))

(event EventRegisterPlayertoRegistry
  (params (Player :type Actor%20Object%20Reference))
  (Game|BindEventtoOnEndPlay Player (delegate Custom|OnPlayerEndplay))
  (bind _returnvalue (Utilities|Array|AddUnique (Variables|Default|GetPlayerArrays) Player))
  (if (!= _returnvalue -1)
    (for _array_element (Variables|Default|GetObservers)
      (Default|OnNewPlayerAdded _array_element Player))))

(event EventRegisterObserver
  (params (Observer :type I%20Game%20State%20Observer%20Interface))
  (Utilities|Array|AddUnique (Variables|Default|GetObservers) Observer))

(fn ConstructionScript)

(fn GetAllCurrentPlayers
  (return (Variables|Default|GetPlayerArrays)))